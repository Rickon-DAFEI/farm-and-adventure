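; BP_Merchant is a clickable merchant character that gives the player access to a store.
; Clicking its capsule creates an OpenStore widget and places it in the viewport at the mouse cursor position.
; Hovering the cursor over the capsule toggles custom depth rendering on the mesh, likely for a highlight or outline effect.
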(event OnBeginCursorOver(CapsuleComponent)
  (params (TouchedComponent :type Primitive%20Component%20Object%20Reference))
  (Rendering|SetRenderCustomDepth (Variables|Character|GetMesh) true))

(event OnEndCursorOver(CapsuleComponent)
  (params (TouchedComponent :type Primitive%20Component%20Object%20Reference))
  (Rendering|SetRenderCustomDepth (Variables|Character|GetMesh) false))

(event OnClicked(CapsuleComponent)
  (params (TouchedComponent :type Primitive%20Component%20Object%20Reference) (ButtonPressed :type Key%20Structure :default "None"))
  (bind _returnvalue (Game|GetPlayerController 0))
  (bind (_locationx _locationy) (Game|Player|GetMousePosition _returnvalue))
  (bind _returnvalue_2 (UserInterface|CreateWidget "/Game/UI/OpenStore.OpenStore_C"))
  (UserInterface|Viewport|AddtoViewport _returnvalue_2 0)
  (Class|UserWidget|SetPositioninViewport _returnvalue_2 (Math|Vector2D|MakeVector2D _locationx _locationy) true))

(event EventBeginPlay)

(event Collision|EventActorBeginOverlap
  (params (OtherActor :type Actor%20Object%20Reference)))

(event EventTick
  (params (DeltaSeconds :type Float%20%28single-precision%29)))

(fn ConstructionScript)